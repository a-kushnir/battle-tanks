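; AC_ProjectileMovement is an actor component that moves its owning projectile in a straight line.
; On BeginPlay it caches the owner's forward vector as the travel direction.
; Each Tick it offsets the owner along that direction by Speed scaled by delta time, with sweep enabled so movement stops at blocking collisions.
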(event `self.ReceiveBeginPlay`
  ;[1 1 1] Constructor
  (set `self.Direcrion` (`Actor.GetActorForwardVector` (`self.GetOwner`))))

(event `self.ReceiveTick`
  (params (DeltaSeconds :type "Float (single-precision)"))
  ;[1 1 1] Movement
  (`Actor.K2_AddActorWorldOffset` (`self.GetOwner`) (* (`self.Direcrion`) (* (`self.Speed`) (`GameplayStatics.GetWorldDeltaSeconds`))) true false))