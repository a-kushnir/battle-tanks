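; Tank movement component for P_Tank that drives grid-aligned running, turning, ice drifting and stopping, plus timed speed-up and slow-down effects.
; The locally controlled tank turns input into state changes, sent through server-to-multicast events that snap remote copies to the sender's transform.
; Every machine then simulates forward motion each tick with a swept offset, scaled by effects and sand, applying forces on wall, box or tank hits.
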(event `self.ReceiveBeginPlay`
  ;[1 1 1] Initialization
  (bind _asp_tank (cast `/Game/LevelGame/Tanks/P_Tank` (`self.GetOwner`)))
  (set `self.Owner Tank` _asp_tank))

(event `self.ReceiveTick`
  (params (DeltaSeconds :type "Float (single-precision)"))
  (`|ExecutionSequence`
    (:`then_0`
      (if (`Pawn.IsLocallyControlled` (`self.Owner Tank`))
        ;[1 1 1] Server Movement
        (`|ExecutionSequence`
          (:`then_0`
            (if (not (`self.Paused`))
              (`/Game/Common/Functions.CountTimerDown` (`self.FreezeTime`))))
          (:`then_1`
            (`self.CheckDirectionChange`)
            (`self.CheckMovementChange`)
            (`self.CheckDriftingChange`)))))
    (:`then_1`
      ;[1 1 1] Speed Effects
      (bind (_enabled _reset) (`/Game/Common/Functions.CountTimerDown` (`self.FastTime`)))
      (if _reset
        (`self.OnSpeedUpEnd`)))
    (:`then_2`
      (bind (_enabled_2 _reset_2) (`/Game/Common/Functions.CountTimerDown` (`self.SlowTime`)))
      (if _reset_2
        (`self.OnSlowDownEnd`)))
    (:`then_3`
      ;[1 1 1] Client Movement
      (if (`|EnumInequality` (`self.Type`) "NewEnumerator2")
        (`self.MovePawn` (`self.GetMovementVector`))))))

(event `Run Server`
  (params (Location :type "Vector Structure") (Rotation :type "Rotator Structure"))
  ;[1 1 1] Starts Movement
  (`self.Run Multicast` Location Rotation))

(event `Run Multicast`
  (params (Location :type "Vector Structure") (Rotation :type "Rotator Structure"))
  ;[1 1 1] Starts Movement
  (`self.UpdateTank` Location Rotation
    (:`Host`
      _)
    (:`Other`
      (set `self.Type` "NewEnumerator0")))
  (set `self.DriftTime` 0.0)
  (`self.OnRunning`))

(event `Drift Server`
  (params (Location :type "Vector Structure") (Rotation :type "Rotator Structure"))
  ;[1 1 1] Slipping
  (`self.Drift Multicast` Location Rotation))

(event `Drift Multicast`
  (params (Location :type "Vector Structure") (Rotation :type "Rotator Structure"))
  ;[1 1 1] Slipping
  (`self.UpdateTank` Location Rotation
    (:`Host`
      _)
    (:`Other`
      (set `self.Type` "NewEnumerator1")))
  (set `self.DriftTime` (`self.DriftInterval`))
  (`self.OnDrifting`))

(event `Stop Server`
  (params (Location :type "Vector Structure") (Rotation :type "Rotator Structure"))
  ;[1 1 1] Stops Movement
  (`self.Stop Multicast` Location Rotation))

(event `Stop Multicast`
  (params (Location :type "Vector Structure") (Rotation :type "Rotator Structure"))
  ;[1 1 1] Stops Movement
  (`self.UpdateTank` Location Rotation
    (:`Host`
      _)
    (:`Other`
      (set `self.Type` "NewEnumerator2")))
  (set `self.DriftTime` 0.0)
  (`self.OnStopped`))

(event `Turn Server`
  (params (Location :type "Vector Structure") (Rotation :type "Rotator Structure"))
  ;[1 1 1] Changes Direction
  (`self.Turn Multicast` Location Rotation))

(event `Turn Multicast`
  (params (Location :type "Vector Structure") (Rotation :type "Rotator Structure"))
  ;[1 1 1] Changes Direction
  (`self.UpdateTank` Location Rotation
    (:`Host`
      _)
    (:`Other`
      _))
  (`self.OnTurned`))

(fn `AdjustCoordinate`
  (params (Coordinate :type "Float (double-precision)"))
  (returns (`Retun Value` :type "Float (double-precision)"))
  (bind _returnvalue (/ (`self.Grid`) 2.0))
  (return (+ (* (`KismetMathLibrary.Round` (/ (- Coordinate _returnvalue) (`self.Grid`))) (`self.Grid`)) _returnvalue)))

(fn `AdjustedLocationAndRotation`
  (returns (Location :type "Vector Structure") (Rotation :type "Rotator Structure"))
  (bind _returnvalue (`Pawn.GetControlRotation` (`self.Owner Tank`)))
  (return (`self.AdjustLocation` (.yaw _returnvalue)) _returnvalue))

(fn `AdjustLocation`
  (params (Rotation :type "Float (double-precision)"))
  (returns (`Retun Value` :type "Vector Structure"))
  (if (== (mod (`KismetMathLibrary.Round` (/ Rotation 90.0)) 2) 0)
    (return (`KismetMathLibrary.MakeVector` (.x (`Actor.K2_GetActorLocation` (`self.Owner Tank`))) (`self.AdjustCoordinate` (.y (`Actor.K2_GetActorLocation` (`self.Owner Tank`)))) (.z (`Actor.K2_GetActorLocation` (`self.Owner Tank`)))))
    (else
      (return (`KismetMathLibrary.MakeVector` (`self.AdjustCoordinate` (.x (`Actor.K2_GetActorLocation` (`self.Owner Tank`)))) (.y (`Actor.K2_GetActorLocation` (`self.Owner Tank`))) (.z (`Actor.K2_GetActorLocation` (`self.Owner Tank`))))))))

(fn `CheckDirectionChange`
  (bind _owner_tank (`self.Owner Tank`))
  (bind _returnvalue (`Pawn.GetControlRotation` (`self.Owner Tank`)))
  (bind _retun_value (`self.AdjustLocation` (.yaw _returnvalue)))
  (if (and (`/Game/LevelGame/Tanks/P_Tank.CanMove?` (`self.Owner Tank`)) (!= (`Actor.K2_GetActorRotation` _owner_tank) (`Pawn.GetControlRotation` _owner_tank)))
    (`Actor.K2_SetActorLocationAndRotation` (`self.Owner Tank`) _retun_value _returnvalue false false)
    (`self.OnTurned`)
    (`self.Turn Server` _retun_value _returnvalue)))

(fn `CheckDriftingChange`
  (bind (_location _rotation) (`self.AdjustedLocationAndRotation`))
  (if (`|EnumEquality` (`self.Type`) "NewEnumerator1")
    (bind _enabled (`/Game/Common/Functions.CountTimerDown` (`self.DriftTime`)))
    (if (not (and _enabled (`self.OnIce?`)))
      (`self.Stop Server` _location _rotation))))

(fn `CheckMovementChange`
  (locals (`Delta Location` :type "Vector Structure"))
  (bind (_location _rotation) (`self.AdjustedLocationAndRotation`))
  (bind (_location_2 _rotation_2) (`self.AdjustedLocationAndRotation`))
  (bind (_location_3 _rotation_3) (`self.AdjustedLocationAndRotation`))
  (`|ExecutionSequence`
    (:`then_0`
      (bind _returnvalue (`Pawn.ConsumeMovementInputVector` (`self.Owner Tank`)))
      (set `local.Delta Location` _returnvalue))
    (:`then_1`
      (if (and (`/Game/LevelGame/Tanks/P_Tank.CanMove?` (`self.Owner Tank`)) (!= (`local.Delta Location`) (0.0 0.0 0.0)))
        (if (`|EnumInequality` (`self.Type`) "NewEnumerator0")
          (set `self.Type` "NewEnumerator0")
          (`self.Run Server` _location _rotation))
        (elif (and (`|EnumEquality` (`self.Type`) "NewEnumerator0") (`self.OnIce?`))
          (set `self.Type` "NewEnumerator1")
          (`self.Drift Server` _location_3 _rotation_3)
          (elif (and (`|EnumInequality` (`self.Type`) "NewEnumerator2") (<= (`self.DriftTime`) 0.0))
            (set `self.Type` "NewEnumerator2")
            (`self.Stop Server` _location_2 _rotation_2)))))))

(fn `GetMovementVector`
  (returns (`Delta Location` :type "Vector Structure"))
  (return (`KismetMathLibrary.GetForwardVector` (`Actor.K2_GetActorRotation` (`self.Owner Tank`)))))

(fn `GetProjectileSpeedFactor`
  (returns (`Speed Factor` :type "Float (double-precision)"))
  (if (> (`self.FastTime`) 0.0)
    (return (`self.FastProjetileSpeedFactor`))
    (elif (> (`self.SlowTime`) 0.0)
      (return (`self.SlowProjetileSpeedFactor`))
      (else
        (return 1.0)))))

(fn `GetTankSpeedFactor`
  (returns (`Speed Factor` :type "Float (double-precision)"))
  (locals (Result :type "Float (double-precision)" :default 1.0))
  (`|ExecutionSequence`
    (:`then_0`
      (if (> (`self.FastTime`) 0.0)
        (set `local.Result` (`self.FastTankSpeedFactor`))
        (elif (> (`self.SlowTime`) 0.0)
          (set `local.Result` (`self.SlowTankSpeedFactor`)))))
    (:`then_1`
      (if (`self.Sandy`)
        (bind (_all_of_them _half_or_more _none_of_them) (`/Game/LevelGame/Tanks/P_Tank.OnWall?` (`self.Owner Tank`) "/Game/Common/Walls/A_SandWall.A_SandWall_C"))
        (set `self.Sandy` (not _none_of_them))
        (if _half_or_more
          (set `local.Result` (* (`local.Result`) 0.5)))))
    (:`then_2`
      (return (`local.Result`)))))

(fn `MovePawn`
  (params (`Delta Location` :type "Vector Structure"))
  (locals (DeltaLocation :type "Vector Structure"))
  (bind _owner_tank (`self.Owner Tank`))
  (bind _sweephitresult (`Actor.K2_AddActorWorldOffset` (`self.Owner Tank`) (* `Delta Location` (* (`GameplayStatics.GetWorldDeltaSeconds`) (`self.GetTankSpeedFactor`) (`self.Speed`))) true false))
  (bind (_bblockinghit _binitialoverlap _time _location _impactpoint _normal _impactnormal _physmat _hitactor) (`GameplayStatics.BreakHitResult` _sweephitresult))
  (cast `/Game/Common/Walls/A_Wall` _hitactor
    (:`then`
      (`/Game/LevelGame/Tanks/P_Tank.ApplyForce` _owner_tank "NewEnumerator3" _hitactor))
    (:`CastFailed`
      (cast `/Game/Common/A_LevelBox` _hitactor
        (:`then`
          (`/Game/LevelGame/Tanks/P_Tank.ApplyForce` _owner_tank "NewEnumerator3" _hitactor))
        (:`CastFailed`
          (cast `/Game/LevelGame/Tanks/P_Tank` _hitactor)
          (`/Game/LevelGame/Tanks/P_Tank.ApplyForce` _owner_tank "NewEnumerator4" _hitactor))))))

(fn `OnIce?`
  (returns (`Return Value` :type Boolean))
  (bind (_all_of_them _half_or_more) (`/Game/LevelGame/Tanks/P_Tank.OnWall?` (`self.Owner Tank`) "/Game/Common/Walls/A_IceWall.A_IceWall_C"))
  (return _half_or_more))

(fn `ResetTimers`
  (set `self.FreezeTime` 0.0)
  (set `self.SlowTime` 0.0)
  (set `self.FastTime` 0.0))

(fn `SlowDown`
  (params (Time :type "Float (double-precision)"))
  (set `self.SlowTime` Time)
  (set `self.FastTime` 0.0)
  (`self.OnSlowDownStart`))

(fn `SpeedUp`
  (params (Time :type "Float (double-precision)"))
  (set `self.FastTime` Time)
  (set `self.SlowTime` 0.0)
  (`self.OnSpeedUpStart`))